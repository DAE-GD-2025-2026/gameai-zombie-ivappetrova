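; BP_Survivor is the survivor actor, which handles incoming damage and pauses the game on death.
; On BeginPlay it registers as a Game Framework Component Manager receiver and binds to its any-damage event.
; Every hit is reported as an AI damage sense event at the causer's location, with zero amount under GodMode.
; Outside GodMode, truncated damage goes to HealthComponent, whose OnDeath event triggers the pause.
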(event `self.ReceiveBeginPlay`
  (`GameFrameworkComponentManager.AddReceiver` (subsystem `GameFrameworkComponentManager`) null true)
  (add `self.OnTakeAnyDamage` (delegate `OnTakeAnyDamage_Event`)))

(event `OnTakeAnyDamage_Event` :!signature `self.OnTakeAnyDamage`
  (params (DamagedActor :type "Actor Object Reference") (Damage :type "Float (single-precision)") (DamageType :type "DamageType Object Reference") (InstigatedBy :type "Controller Object Reference") (DamageCauser :type "Actor Object Reference"))
  (bind _returnvalue (select `bool` (`self.GodMode`) :`false` Damage))
  (`AISense_Damage.ReportDamageEvent` self DamageCauser _returnvalue (`self.K2_GetActorLocation` DamageCauser) (0.0 0.0 0.0) "Damage")
  (if (not (`self.GodMode`))
    (`HealthComponent.TakeDamage` (`self.HealthComponent`) (`KismetMathLibrary.FTrunc` _returnvalue))))

(event `self.HealthComponent.OnDeath`
  (`GameplayStatics.SetGamePaused` true))

(fn `UserConstructionScript`)